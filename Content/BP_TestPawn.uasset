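; BP_TestPawn is a test pawn that drives a dialogue system, BPTestDialogue, from player input.
; Start and Continue input actions begin the interview and advance it.
; Input actions 1 to 4 select the matching dialogue choice by zero-based index.
; The pawn holds no other logic, and its construction script is empty.
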(event Input|ActionEvents|InputActionStart
  (params (Key :type Key%20Structure :default "None"))
  (:Pressed
    (Class|DialogueComponent|StartInterview (Variables|Default|GetBP_TestDialogue))))

(event Input|ActionEvents|InputActionContinue
  (params (Key :type Key%20Structure :default "None"))
  (:Pressed
    (Class|DialogueComponent|Continue (Variables|Default|GetBP_TestDialogue))))

(event Input|ActionEvents|InputAction1
  (params (Key :type Key%20Structure :default "None"))
  (:Pressed
    (Class|DialogueComponent|Select (Variables|Default|GetBP_TestDialogue))))

(event Input|ActionEvents|InputAction2
  (params (Key :type Key%20Structure :default "None"))
  (:Pressed
    (Class|DialogueComponent|Select (Variables|Default|GetBP_TestDialogue) 1)))

(event Input|ActionEvents|InputAction3
  (params (Key :type Key%20Structure :default "None"))
  (:Pressed
    (Class|DialogueComponent|Select (Variables|Default|GetBP_TestDialogue) 2)))

(event Input|ActionEvents|InputAction4
  (params (Key :type Key%20Structure :default "None"))
  (:Pressed
    (Class|DialogueComponent|Select (Variables|Default|GetBP_TestDialogue) 3)))

(fn ConstructionScript)