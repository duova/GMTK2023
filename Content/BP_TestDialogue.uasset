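; BP_TestDialogue is the presentation handler for an interview game where the player asks questions and guesses a character's career.
; Dialogue events cache questions, answers, meter value and career options in variables, then add the matching widget to the viewport, with debug prints throughout.
; A correct ending increments the game mode's WinCount, plays applause and reloads TestMap after a delay.
; A bust or wrong guess shows failure and resets WinCount and SusMeter.
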(event EventOnUIClear
  (Development|PrintString "UI cleared"))

(event EventOnDisplayAnswer
  (params (Answer :type Text%20%28by%20ref%29) (NewMeterValueInDecimal :type Float%20%28single-precision%29))
  (Development|PrintString (Utilities|String|ToString(Text) Answer) true true "(R=0.000000,G=0.660000,B=1.000000,A=1.000000)" 5.0)
  (Development|PrintString (Utilities|String|Append "Meter Value: " (Utilities|String|ToString(Float) NewMeterValueInDecimal)))
  (Variables|Default|SetNew%20Meter%20Value%20in%20Decimal NewMeterValueInDecimal)
  (Variables|Default|SetAnswer Answer)
  (bind _returnvalue (UserInterface|CreateWidget "/Game/UI/UserInterface/UI_Widget_Answer.UI_Widget_Answer_C"))
  (UserInterface|Viewport|AddtoViewport _returnvalue 0))

(event EventOnDisplayBust
  (params (BustText :type Text%20%28by%20ref%29))
  (Development|PrintString (Utilities|String|ToString(Text) BustText))
  (bind _returnvalue (UserInterface|CreateWidget "/Game/UI/UserInterface/UI_Widget_Failure.UI_Widget_Failure_C"))
  (UserInterface|Viewport|AddtoViewport _returnvalue 0)
  (bind _asbp_test_game_mode (Utilities|Casting|CastToBP_TestGameMode (Game|GetGameMode)))
  (Variables|/Game/BP_TestGameMode.BP_TestGameMode_C|SetWin%20Count _asbp_test_game_mode 0)
  (Variables|/Game/BP_TestGameMode.BP_TestGameMode_C|SetSusMeter _asbp_test_game_mode 0))

(event EventOnDisplayEndingText
  (params (EndingText :type Text%20%28by%20ref%29) (bCorrect :type Boolean))
  (Development|PrintString (Utilities|String|ToString(Text) EndingText) true true "(R=0.000000,G=0.660000,B=1.000000,A=1.000000)" 5.0)
  (Development|PrintString (Utilities|String|Append "Has Won:" (Utilities|String|ToString(Boolean) bCorrect)))
  (if bCorrect
    (bind _returnvalue (UserInterface|CreateWidget "/Game/UI/UserInterface/UI_Widget_Success.UI_Widget_Success_C"))
    (UserInterface|Viewport|AddtoViewport _returnvalue 0)
    (bind _asbp_test_game_mode (Utilities|Casting|CastToBP_TestGameMode (Game|GetGameMode)))
    (Variables|/Game/BP_TestGameMode.BP_TestGameMode_C|SetWin%20Count _asbp_test_game_mode (+ (Variables|/Game/BP_TestGameMode.BP_TestGameMode_C|GetWin%20Count _asbp_test_game_mode) 1))
    (Audio|PlaySound2D "/Game/Audio/Interview_audio_applause_Cue.Interview_audio_applause_Cue" 1.0 1.0 0.0 0 0)
    (Utilities|FlowControl|Delay 5.0)
    (Game|OpenLevel(byName) "TestMap")
    (else
      (bind _returnvalue_2 (UserInterface|CreateWidget "/Game/UI/UserInterface/UI_Widget_Failure.UI_Widget_Failure_C"))
      (UserInterface|Viewport|AddtoViewport _returnvalue_2 0)
      (bind _asbp_test_game_mode_2 (Utilities|Casting|CastToBP_TestGameMode (Game|GetGameMode)))
      (Variables|/Game/BP_TestGameMode.BP_TestGameMode_C|SetWin%20Count _asbp_test_game_mode_2 0)
      (Variables|/Game/BP_TestGameMode.BP_TestGameMode_C|SetSusMeter _asbp_test_game_mode_2 0))))

(event EventOnDisplayQuestions
  (params (QuestionOptions :type Array%20of%20Texts))
  ;[1 1 1] Questions
  (Variables|Default|SetQuestion_1 (Utilities|Array|Get(acopy) QuestionOptions))
  (Variables|Default|SetQuestion_2 (Utilities|Array|Get(acopy) QuestionOptions 1))
  (Variables|Default|SetQuestion_3 (Utilities|Array|Get(acopy) QuestionOptions 2))
  (Variables|Default|SetQuestion_4 (Utilities|Array|Get(acopy) QuestionOptions 3))
  (bind _returnvalue (UserInterface|CreateWidget "/Game/UI/UserInterface/UI_Widget_Questions.UI_Widget_Questions_C"))
  (UserInterface|Viewport|AddtoViewport _returnvalue 0))

(event EventOnInterviewEnd
  (Development|PrintString "Interview Ended"))

(event EventOnInterviewStart
  (params (StartingText :type Text%20%28by%20ref%29))
  (Development|PrintString (Utilities|String|ToString(Text) StartingText)))

(event EventOnDisplayOptions
  (params (CharacterTitleOptions :type Array%20of%20Texts))
  ;[1 1 1] Choose career
  (Variables|Default|SetCareer_1 (Utilities|Array|Get(acopy) CharacterTitleOptions))
  (Variables|Default|SetCareer_2 (Utilities|Array|Get(acopy) CharacterTitleOptions 1))
  (Variables|Default|SetCareer_3 (Utilities|Array|Get(acopy) CharacterTitleOptions 2))
  (Variables|Default|SetCareer_4 (Utilities|Array|Get(acopy) CharacterTitleOptions 3))
  (Variables|Default|SetCareer_5 (Utilities|Array|Get(acopy) CharacterTitleOptions 4))
  (bind _returnvalue (UserInterface|CreateWidget "/Game/UI/UserInterface/UI_Widget_Guess.UI_Widget_Guess_C"))
  (UserInterface|Viewport|AddtoViewport _returnvalue 0))